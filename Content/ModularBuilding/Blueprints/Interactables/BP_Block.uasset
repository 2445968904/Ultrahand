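; BP_Block is a modular building piece that is grabbed with a physics handle, dropped, or attached to another block.
; Attached blocks form a hierarchy, propagating child-list changes up through parents and recursing collision updates and overlap checks down through children.
; While held, it switches collision to overlap and shows a red hologram material on overlap, except during rotation.
; Snap points are stored in parallel arrays, re-sorted by priority on each addition.
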(event `self.StaticMesh.OnComponentSleep`
  (params (SleepingComponent :type "PrimitiveComponent Object Reference") (BoneName :type Name))
  ;[1 1 1] Physics Related
  (`PrimitiveComponent.WakeRigidBody` (`self.StaticMesh`) "None"))

(event `self.ReceiveBeginPlay`
  ;[0 0 0] BeginPlay
  ;;[0.2089 0.1844 1] Cache Starting Material
  (set `self.Cached Material` (`PrimitiveComponent.GetMaterial` (`self.StaticMesh`) 0))
  (`SceneComponent.SetWorldScale3D` (`self.StaticMesh`) (`KismetMathLibrary.Conv_DoubleToVector` (`self.scale`))))

(event `Change Scale`
  (params (Place :type Boolean))
  ;[1 0.6799 0.2575] Lerp Actor Scale When Picked Up / Put Down
  (if Place
    (bind (_direction _alpha) (`Timeline|Timeline_Scale` :!via `ReverseFromEnd` :!label _label)
      (:`Update`
        (`self.SetActorScale3D` (`KismetMathLibrary.Conv_DoubleToVector` (* _alpha (`self.scale`))))))
    (else
      (goto _label :!via `PlayFromStart`))))

(event `self.ReceiveTick`
  (params (DeltaSeconds :type "Float (single-precision)"))
  (bind _cached_material (`self.Cached Material`))
  ;[0 0 0] Tick
  ;;[1 0.1968 0.3268] Update Material If Overlapping
  (if (`self.PickedUp`)
    (if (not (`self.IsRotating?`))
      (`PrimitiveComponent.SetMaterial` (`self.StaticMesh`) 0 (select `bool` (== (`KismetArrayLibrary.Array_Length` (`PrimitiveComponent.GetOverlappingActors` (`self.StaticMesh`) "/Script/Engine.Actor")) 0) :`false` "/Game/ModularBuilding/Assets/Materials/Master/MI_ProcGrid_Hologram_Red.MI_ProcGrid_Hologram_Red" :`true` _cached_material))
      (else
        (`PrimitiveComponent.SetMaterial` (`self.StaticMesh`) 0 _cached_material :!label _label_2)))
    (else
      (goto _label_2))))

(event `self.Add Snap Point`
  (params (Location :type "Vector Structure") (Rotation :type "Rotator Structure") (Priority :type Integer))
  ;[0.3458 0.9001 1] Interface
  ;;[1 1 1] Add Snap Point
  (`KismetArrayLibrary.Array_Add` (`self.Snap Points`) Location)
  (`KismetArrayLibrary.Array_Add` (`self.Snap Directions`) Rotation)
  (`KismetArrayLibrary.Array_Add` (`self.Snap Priority`) Priority)
  (`self.Snap Apply Priority`))

(event `self.Pickup`
  (params (`Physics Handle` :type "PhysicsHandleComponent Object Reference"))
  (bind (_returnvalue_location _returnvalue_rotation) (`KismetMathLibrary.BreakTransform` (`self.GetTransform`)))
  (bind _staticmesh (`self.StaticMesh`))
  ;[0 0 0] Pickup
  (`|ExecutionSequence`
    (:`then_0`
      (`/Engine/EditorBlueprintResources/StandardMacros.IsValid` `Physics Handle`
        (:`Is Valid`
          (`self.Remove`)
          (`PhysicsHandleComponent.GrabComponentAtLocationWithRotation` `Physics Handle` (`self.StaticMesh`) "None" _returnvalue_location _returnvalue_rotation)
          (bind _output_get (set `self.PickedUp` true))
          (`self.Change Scale` _output_get))))
    (:`then_1`
      (`PrimitiveComponent.SetCollisionResponseToChannel` _staticmesh "ECC_PhysicsBody" "ECR_Overlap")
      (`PrimitiveComponent.SetCollisionResponseToChannel` _staticmesh "ECC_WorldStatic" "ECR_Overlap")
      (`self.CloseCollision`)
      ;;[1 0.3851 0.7828] Call On Children
      (bind _array_element (`self.Call On Children`)
        (:`LoopBody`
          (bind _asbp_block (cast `/Game/ModularBuilding/Blueprints/Interactables/BP_Block` _array_element))
          (`self.Child Collision Update` _asbp_block "QueryOnly"))))))

(event `self.Add Child`
  (params (`Child Actor` :type "Actor Object Reference"))
  ;[0.3458 0.9001 1] Interface
  ;;[1 1 1] Add Child
  (`KismetArrayLibrary.Array_Add` (`self.Child Actors`) `Child Actor`)
  (message `/Game/ModularBuilding/Blueprints/Core/BPI_ModularBuilding.Add Child` (`self.Parent`) `Child Actor`))

(event `self.TransferChildren`
  (params (`Child Actors` :type "Array of Actor Object Reference (by ref)"))
  ;[0.3458 0.9001 1] Interface
  ;;[1 1 1] Add Child
  (for _array_element `Child Actors`
    (`self.Add Child` _array_element)))

(event `self.Remove Child`
  (params (Actor :type "Actor Object Reference"))
  ;[0.3458 0.9001 1] Interface
  ;;[1 1 1] Remove Child
  (`KismetArrayLibrary.Array_RemoveItem` (`self.Child Actors`) Actor)
  (message `/Game/ModularBuilding/Blueprints/Core/BPI_ModularBuilding.Remove Child` (`self.Parent`) Actor))

(event `self.Drop`
  (params (`Physics Handle` :type "PhysicsHandleComponent Object Reference"))
  (bind _staticmesh (`self.StaticMesh`))
  ;[0 0 0] Drop
  (`/Engine/EditorBlueprintResources/StandardMacros.IsValid` `Physics Handle`
    (:`Is Valid`
      (`PhysicsHandleComponent.ReleaseComponent` `Physics Handle`))
    (:`Is Not Valid`
      _))
  (set `self.PickedUp` false)
  (`self.Change Scale` false)
  (`PrimitiveComponent.SetCollisionResponseToChannel` _staticmesh "ECC_PhysicsBody" "ECR_Block")
  (`PrimitiveComponent.SetCollisionResponseToChannel` _staticmesh "ECC_WorldStatic" "ECR_Block")
  (`PrimitiveComponent.SetCollisionEnabled` _staticmesh "QueryAndPhysics")
  ;;[1 0.3851 0.7828] Call On Children
  (bind _array_element (`self.Call On Children`)
    (:`LoopBody`
      (bind _asbp_block (cast `/Game/ModularBuilding/Blueprints/Interactables/BP_Block` _array_element))
      (`self.Child Collision Update` _asbp_block "QueryAndPhysics"))))

(event `self.RemoveChildren`
  (params (Children :type "Array of Actor Object Reference (by ref)"))
  ;[0.3458 0.9001 1] Interface
  ;;[1 1 1] Remove Child
  (for _array_element Children
    (`self.Remove Child` _array_element)))

(event `self.Rotation Collision Temp Suspend`
  ;[0.3458 0.9001 1] Interface
  ;;[1 1 1] Visual: Collision Check When Rotating
  (set `self.IsRotating?` true)
  (`Timeline|Timeline_RotateVisual` :!via `PlayFromStart`
    (:`Finished`
      (set `self.IsRotating?` false))))

(event `self.Place`
  (params (`Attach To` :type "Actor Object Reference") (`World Transform` :type "Transform Structure"))
  (bind _staticmesh (`self.StaticMesh`))
  ;[0 0 0] Place
  (message `/Game/ModularBuilding/Blueprints/Core/BPI_ModularBuilding.Add Child` `Attach To` self)
  (`self.K2_AttachToActor` self `Attach To` "None" "KeepWorld" "SnapToTarget" "KeepWorld" true)
  (`PrimitiveComponent.SetSimulatePhysics` (`self.StaticMesh`) false)
  (set `self.Parent` `Attach To`)
  (`self.K2_SetActorRelativeLocation` (.location `World Transform`))
  (`self.K2_SetActorRotation` (.rotation `World Transform`))
  (message `/Game/ModularBuilding/Blueprints/Core/BPI_ModularBuilding.TransferChildren` `Attach To` (`self.Child Actors`))
  (`PrimitiveComponent.SetCollisionResponseToChannel` _staticmesh "ECC_PhysicsBody" "ECR_Block")
  (`PrimitiveComponent.SetCollisionResponseToChannel` _staticmesh "ECC_WorldStatic" "ECR_Block")
  (`PrimitiveComponent.SetCollisionEnabled` _staticmesh "QueryAndPhysics")
  ;;[1 0.3851 0.7828] Call On Children
  (bind _array_element (`self.Call On Children`)
    (:`LoopBody`
      (bind _asbp_block (cast `/Game/ModularBuilding/Blueprints/Interactables/BP_Block` _array_element))
      (`self.Child Collision Update` _asbp_block "QueryAndPhysics"))
    (:`Completed`
      ;[1 0.6119 0.2157] Sound: Place
      (`GameplayStatics.PlaySound2D` "/Game/ModularBuilding/Assets/Sounds/Technology_Pickup_Cue.Technology_Pickup_Cue" 0.2 1.0 0.035 null null)
      (`self.OpenCollision`)
      (bind _asbp_block_2 (cast `/Game/ModularBuilding/Blueprints/Interactables/BP_Block` `Attach To`))
      (`self.UpdateBodyConnection` _asbp_block_2))))

(event `self.Remove`
  (bind _parent (`self.Parent`))
  ;[0 0 0] Remove
  (`self.K2_DetachFromActor` "KeepWorld" "KeepWorld" "KeepWorld")
  (`PrimitiveComponent.SetSimulatePhysics` (`self.StaticMesh`) true)
  (message `/Game/ModularBuilding/Blueprints/Core/BPI_ModularBuilding.Remove Child` _parent self)
  (message `/Game/ModularBuilding/Blueprints/Core/BPI_ModularBuilding.RemoveChildren` _parent (`self.Child Actors`))
  (set `self.Parent` null))

(event `Child Collision Update`
  (params (NewType :type "ECollisionEnabled Enum" :default "NoCollision"))
  (bind _returnvalue (select `ECollisionEnabled` NewType :`NoCollision` "ECR_Overlap" :`QueryOnly` "ECR_Overlap" :`PhysicsOnly` "ECR_Ignore" :`QueryAndPhysics` "ECR_Block" :`ProbeOnly` "ECR_Ignore" :`QueryAndProbe` "ECR_Ignore" :!type "ECollisionResponse Enum"))
  (bind _staticmesh (`self.StaticMesh`))
  ;[0.9713 0.3431 1] Update Child Actor Collision
  (`PrimitiveComponent.SetCollisionEnabled` _staticmesh NewType)
  (`PrimitiveComponent.SetCollisionResponseToChannel` _staticmesh "ECC_PhysicsBody" _returnvalue)
  (`PrimitiveComponent.SetCollisionResponseToChannel` _staticmesh "ECC_WorldStatic" _returnvalue)
  (set `self.PickedUp` (select `ECollisionEnabled` NewType :`NoCollision` true :`QueryOnly` true))
  (bind _array_element (`self.Call On Children`)
    (:`LoopBody`
      (bind _asbp_block (cast `/Game/ModularBuilding/Blueprints/Interactables/BP_Block` _array_element))
      (`self.Child Collision Update` _asbp_block NewType))))

(event `self.UpdateBodyConnection`
  (params (Actor :type "/Game/ModularBuilding/Blueprints/Interactables/BP_Block Object Reference")))

(fn `CloseCollision`
  (for _array_element (`self.GetAllOwnerStaticComponent`)
    (if (!= (`self.StaticMesh`) _array_element)
      (`PrimitiveComponent.SetCollisionResponseToChannel` _array_element "ECC_WorldStatic" "ECR_Ignore")
      (`PrimitiveComponent.SetCollisionResponseToChannel` _array_element "ECC_WorldDynamic" "ECR_Ignore")
      (`PrimitiveComponent.SetCollisionResponseToChannel` _array_element "ECC_PhysicsBody" "ECR_Ignore"))))

(fn `Get Children`
  (returns (Children :type "Array of Actor Object Reference"))
  (return (`self.Child Actors`)))

(fn `Get Connection Size`
  (returns (`Connection Size` :type Integer))
  (return (`self.Connection Size`)))

(fn `Get Snap Directions`
  (returns (`Snap Directions` :type "Array of Rotator Structure"))
  (return (`self.Snap Directions`)))

(fn `Get Snap Points`
  (returns (`Snap Points` :type "Array of Vector Structure"))
  (return (`self.Snap Points`)))

(fn `GetAllOwnerStaticComponent`
  (returns (ReturnValue :type "Array of StaticMeshComponent Object Reference"))
  (return (`self.K2_GetComponentsByClass` "/Script/Engine.StaticMeshComponent")))

(fn `OpenCollision`
  (for _array_element (`self.GetAllOwnerStaticComponent`)
    (if (!= (`self.StaticMesh`) _array_element)
      (`PrimitiveComponent.SetCollisionResponseToChannel` _array_element "ECC_WorldStatic" "ECR_Block"))))

(fn `Overlap Check`
  (returns (Status :type Boolean))
  (locals (`Valid Placement` :type Boolean))
  (set `local.Valid Placement` (== (`KismetArrayLibrary.Array_Length` (`PrimitiveComponent.GetOverlappingActors` (`self.StaticMesh`) "/Script/Engine.Actor")) 0))
  (bind _array_element (`self.Call On Children`)
    (:`LoopBody`
      (bind _status (message `/Game/ModularBuilding/Blueprints/Core/BPI_ModularBuilding.Overlap Check` _array_element))
      (if (not _status)
        (set `local.Valid Placement` false)))
    (:`Completed`
      (return (`local.Valid Placement`)))))

(fn `ParentCheck`
  (returns (Result :type Boolean))
  (return (> (`KismetArrayLibrary.Array_Length` (`self.Child Actors`)) 0)))

(fn `Snap Apply Priority`
  (locals (`Temp Snap Points` :type "Array of Vector Structure") (`Temp Snap Directions` :type "Array of Rotator Structure") (`Temp Snap Priority` :type "Array of Integer") (`Index (local)` :type Integer) (`Min Index (local)` :type Integer :default 0))
  (bind _snap_priority (`self.Snap Priority`))
  ;[0.2215 0.682 1] Loop Through All Snap Points
  (for _index (range (`KismetArrayLibrary.Array_Length` _snap_priority))
    ;[1 1 1] Set Local Variables
    (set `local.Index (local)` _index)
    (set `local.Min Index (local)` (`KismetMathLibrary.MinOfIntArray` _snap_priority))
    ;[0.8133 0.3254 1] Add To Temp
    (`KismetArrayLibrary.Array_Set` (`local.Temp Snap Points`) (`local.Index (local)`) (`|GetArrayItem` (`self.Snap Points`) (`local.Min Index (local)`)) true)
    (`KismetArrayLibrary.Array_Set` (`local.Temp Snap Directions`) (`local.Index (local)`) (`|GetArrayItem` (`self.Snap Directions`) (`local.Min Index (local)`)) true)
    (`KismetArrayLibrary.Array_Set` (`local.Temp Snap Priority`) (`local.Index (local)`) (`|GetArrayItem` (`self.Snap Priority`) (`local.Min Index (local)`)) true)
    ;[1 0.2806 0.1808] Set to Max Int
    (`KismetArrayLibrary.Array_Set` (`self.Snap Priority`) (`local.Min Index (local)`) 2147483647))
  ;[0.2575 1 0.3087] Save Temp Values
  (set `self.Snap Points` (`local.Temp Snap Points`))
  (set `self.Snap Directions` (`local.Temp Snap Directions`))
  (set `self.Snap Priority` (`local.Temp Snap Priority`)))

(fn `Update On Pickup`)

(fn `UserConstructionScript`)