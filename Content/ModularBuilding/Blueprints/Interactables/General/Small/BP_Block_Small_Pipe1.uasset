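; Small pipe block for the modular building system, with a wheel jointed to its cylinder body.
; The construction script runs the parent's, then binds Wheel to Cylinder through the WheelSuspension and WheelAxis physics constraints.
; UpdateBodyConnection adds a physics constraint component to the passed actor at runtime, joining Cylinder to that actor's StaticMesh with all linear and angular motion locked as a rigid weld.
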(event `self.UpdateBodyConnection`
  (params (Actor :type "/Game/ModularBuilding/Blueprints/Interactables/BP_Block Object Reference"))
  (bind _returnvalue (`|AddComponentByClass` :`self` Actor :`Class` "/Script/Engine.PhysicsConstraintComponent"))
  (`PhysicsConstraintComponent.SetConstrainedComponents` _returnvalue (`self.Cylinder`) "None" (`/Game/ModularBuilding/Blueprints/Interactables/BP_Block.StaticMesh` Actor) "None")
  (`PhysicsConstraintComponent.SetLinearXLimit` _returnvalue "LCM_Locked" 0.0)
  (`PhysicsConstraintComponent.SetLinearYLimit` _returnvalue "LCM_Locked" 0.0)
  (`PhysicsConstraintComponent.SetLinearZLimit` _returnvalue "LCM_Locked" 0.0)
  (`PhysicsConstraintComponent.SetAngularTwistLimit` _returnvalue "ACM_Locked" 0.0)
  (`PhysicsConstraintComponent.SetAngularSwing1Limit` _returnvalue "ACM_Locked" 0.0)
  (`PhysicsConstraintComponent.SetAngularSwing2Limit` _returnvalue "ACM_Locked" 0.0))

(fn `UserConstructionScript`
  (`parent.UserConstructionScript`)
  (`PhysicsConstraintComponent.SetConstrainedComponents` (`self.WheelSuspension`) (`self.Wheel`) "None" (`self.Cylinder`) "None")
  (`PhysicsConstraintComponent.SetConstrainedComponents` (`self.WheelAxis`) (`self.Wheel`) "None" (`self.Cylinder`) "None"))